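; Plumber character Blueprint that drives movement head bob and contains footstep sound logic.
; Each tick, once CanStartGame is set, velocity selects an idle, walk or sprint camera shake and stops or plays the footstep timeline at a matching rate.
; A downward sphere trace gates a water footstep sound, but the timeline handler that calls it never runs.
; SprayHitBox overlap only prints a debug string.
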(event `self.ReceiveTick`
  (params (DeltaSeconds :type "Float (single-precision)"))
  (`self.HeadBob`))

(event `HeadBob`
  (bind _returnvalue (`GameplayStatics.GetPlayerController` 0))
  (bind _footsteps_tl (`self.FootSteps_TL`))
  (bind _footsteps_tl_2 (`self.FootSteps_TL`))
  (bind _returnvalue_2 (`KismetMathLibrary.VSize` (`self.GetVelocity`)))
  ;[1 1 1] HeadBob and footsteps
  (if (`self.CanStartGame`)
    (if (> _returnvalue_2 0.0)
      (if (< _returnvalue_2 400.0)
        (`PlayerController.ClientStartCameraShake` :`self` _returnvalue :`Shake` "/Game/HeadBob/CS_Walk.CS_Walk_C")
        (`TimelineComponent.SetPlayRate` _footsteps_tl_2 1.0)
        (`TimelineComponent.Play` _footsteps_tl_2)
        (else
          (`PlayerController.ClientStartCameraShake` :`self` _returnvalue :`Shake` "/Game/HeadBob/CS_Sprint.CS_Sprint_C")
          (`TimelineComponent.SetPlayRate` _footsteps_tl 2.0)
          (`TimelineComponent.Play` _footsteps_tl)))
      (else
        (`TimelineComponent.Stop` (`self.FootSteps_TL`))
        (`PlayerController.ClientStartCameraShake` :`self` _returnvalue :`Shake` "/Game/HeadBob/CS_Idle.CS_Idle_C")))))

(event `self.SprayHitBox.OnComponentBeginOverlap`
  (params (OverlappedComponent :type "PrimitiveComponent Object Reference") (OtherActor :type "Actor Object Reference") (OtherComp :type "PrimitiveComponent Object Reference") (OtherBodyIndex :type Integer) (bFromSweep :type Boolean) (SweepResult :type "HitResult Structure (by ref)"))
  (`KismetSystemLibrary.PrintString` "Hello"))

(fn `footstepTry`
  (bind _finished (`self.TraceFootsteps`))
  (if _finished
    (`GameplayStatics.PlaySoundAtLocation` "/Game/Sounds/Wet/SC_Water.SC_Water" (`self.K2_GetActorLocation`) (struct) 1.0 1.0 0.0 null null null null)))

(fn `TraceFootsteps`
  (returns (Finished :type Boolean))
  (bind _returnvalue (`self.K2_GetActorLocation`))
  (bind _capsulecomponent (`self.CapsuleComponent`))
  (bind (_outhit _returnvalue_2) (`KismetSystemLibrary.SphereTraceSingle` _returnvalue (`KismetMathLibrary.MakeVector` (.x _returnvalue) (.y _returnvalue) (- (.z _returnvalue) (`CapsuleComponent.GetScaledCapsuleHalfHeight` _capsulecomponent))) (`CapsuleComponent.GetScaledCapsuleRadius` _capsulecomponent) "TraceTypeQuery1"))
  (return _returnvalue_2))

(fn `UserConstructionScript`)