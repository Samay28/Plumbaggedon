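; BP_BgMusic is an actor that switches the background music according to whether all valves are closed.
; Each tick it finds a BP_Valve actor, reads AllValvesClosed, and sets the Bg sound to Ready_Aim_Fire when true or Tunnel_ambience otherwise.
; One flag per track limits each sound assignment to a single time, and neither flag is ever reset.
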(event `self.ReceiveBeginPlay`)

(event `self.ReceiveTick`
  (params (DeltaSeconds :type "Float (single-precision)"))
  (bind _bg (`self.bg`))
  (bind _returnvalue (`GameplayStatics.GetActorOfClass` "/Game/Blueprints/Actors/BP_Valve.BP_Valve_C"))
  (if (`Valve.AllValvesClosed` _returnvalue)
    (if (not (`self.IsSetMetal`))
      (`AudioComponent.SetSound` _bg "/Game/Sounds/BG/Ready_Aim_Fire.Ready_Aim_Fire")
      (set `self.IsSetMetal` true))
    (elif (not (`self.IsSetAmbience`))
      (`AudioComponent.SetSound` _bg "/Game/Sounds/BG/tunnel_ambience.tunnel_ambience")
      (set `self.IsSetAmbience` true))))

(fn `UserConstructionScript`)