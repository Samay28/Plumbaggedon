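; BP_Ladder is a ladder actor that ends the game when the plumber character overlaps it.
; On overlap it destroys all BP_Enemy actors, clears all widgets and shows the WBP_Credits screen.
; It disables the player's input, waits through a fixed delay, then reloads or opens MainMap.
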(event `self.ReceiveActorBeginOverlap`
  (params (OtherActor :type "Actor Object Reference"))
  (bind _asbp_plumber_character (cast `/Game/Blueprints/BP_PlumberCharacter` OtherActor))
  (bind _outactors (`GameplayStatics.GetAllActorsOfClass` "/Game/Blueprints/Enemy/BP_Enemy.BP_Enemy_C"))
  (`self.K2_DestroyActor` _outactors)
  (`WidgetLayoutLibrary.RemoveAllWidgets`)
  (bind _returnvalue (`|CreateWidget` "/Game/UI/WBP_Credits.WBP_Credits_C"))
  (`UserWidget.AddToViewport` _returnvalue 0)
  (`self.DisableInput` _asbp_plumber_character (`GameplayStatics.GetPlayerController` 0))
  (`KismetSystemLibrary.Delay` 10.0)
  (`GameplayStatics.OpenLevel` "MainMap"))

(fn `UserConstructionScript`)